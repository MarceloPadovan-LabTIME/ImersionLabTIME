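; BP_MainPlayerCharacter is the player character Blueprint, which drives a dynamic on-screen crosshair that spreads with movement speed.
; On BeginPlay it creates a WBCrosshair widget, stores the reference and adds it to the viewport.
; Each Tick it maps velocity magnitude through a clamped range and writes the result to the widget's CrosshairSpread, widening the crosshair as the character moves faster.
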(event EventBeginPlay
  ;[1 1 1] Add crosshair to screen
  (Utilities|FlowControl|Sequence
    (:then_0
      (bind _returnvalue (UserInterface|CreateWidget "/Game/Art/Crosshair/DynamicCrossHair.WBCrosshair_C"))
      (bind _output_get (Variables|Default|SetCrosshair _returnvalue))
      (UserInterface|Viewport|AddtoViewport _output_get 0))))

(event EventTick
  (params (DeltaSeconds :type Float%20%28single-precision%29))
  ;[1 1 1] Dynamically change the crosshair spread while walk
  (Utilities|FlowControl|Sequence
    (:then_0
      (Variables|/Game/Art/Crosshair/DynamicCrossHair.WBCrosshair_C|Setcrosshair_spread (Variables|Default|GetCrosshair) (Math|Float|MapRangeClamped (Math|Vector|VectorLength (Transformation|GetVelocity)) 0.0 2e+02 5.0 2e+01)))))

(fn ConstructionScript)